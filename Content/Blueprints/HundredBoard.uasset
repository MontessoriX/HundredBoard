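; HundredBoard builds a hundred-square board of DropTarget actors, numbered 1 to 100.
; On BeginPlay, nested loops spawn a ten-by-ten grid of evenly spaced targets, owned by the board, and set each Id row by row.
; Positions are fixed world coordinates centred on the origin in X and Y, so they ignore the board's own transform.
; The construction script is empty.
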(event EventBeginPlay
  (for _index (range 1 10)
    (for _index_2 (range 1 10)
      (bind _returnvalue (Game|SpawnActorfromClass "/Game/Blueprints/DropTarget.DropTarget_C" (Math|Transform|MakeTransform (Math|Vector|MakeVector (Math|Conversions|ToFloat(Integer) (+ (* _index -100) 550)) (Math|Conversions|ToFloat(Integer) (+ (* _index_2 100) -550)) 5e+01)) "AlwaysSpawn" self 0))
      (Variables|/Game/Blueprints/DropTarget.DropTarget_C|Setid _returnvalue (+ (* (- _index 1) 10) _index_2)))))

(fn ConstructionScript)