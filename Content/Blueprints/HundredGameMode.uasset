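; HundredGameMode is the game mode for a number-tile game, feeding in numbered pieces ten at a time.
; On BeginPlay, CreateTenTiles spawns ten consecutively numbered NumberPiece actors at random positions and slight random yaw within a fixed area, tracking the last number and count in play.
; CorrectlyDropTile decrements that count and, when it empties, prints the current number and spawns the next ten, with no upper limit checked here.
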(event EventBeginPlay
  (CallFunction|CreateTenTiles (Variables|Default|GetcurrentNumber)))

(fn ConstructionScript)

(fn CreateTenTiles
  (params (startingID :type Integer))
  (for _index (range startingID (+ startingID 9))
    (bind _returnvalue (Game|SpawnActorfromClass "/Game/Blueprints/NumberPiece.NumberPiece_C" (Math|Transform|MakeTransform (Math|Vector|MakeVector (Math|Random|RandomFloatinRange -4.3e+02 4.3e+02) (Math|Random|RandomFloatinRange 5.7e+02 1.14e+03) 3e+01) (Math|Rotator|MakeRotator 0.0 0.0 (Math|Random|RandomFloatinRange -1e+01 1e+01)) "0.980000,0.980000,0.100000") "AdjustIfPossibleButAlwaysSpawn" 0 0))
    (Default|SetID _returnvalue _index)
    (Variables|Default|SetcurrentNumber _index))
  (Variables|Default|SetnumInPlay (+ (Variables|Default|GetnumInPlay) 10)))

(fn CorrectlyDropTile
  (bind _currentnumber (Variables|Default|GetcurrentNumber))
  (Variables|Default|SetnumInPlay (- (Variables|Default|GetnumInPlay) 1))
  (if (< (Variables|Default|GetnumInPlay) 1)
    (Development|PrintString (Utilities|String|ToString(Integer) _currentnumber))
    (CallFunction|CreateTenTiles (+ _currentnumber 1))))